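; A 2D Paper2D flipbook character that moves along the X and Z axes from the RightOrLeft and UpOrDown input axes.
; Each tick, SetMyFlipbook stores the last input direction, with vertical input taking priority over horizontal.
; It then picks a directional move or idle flipbook based on whether velocity is nonzero, so idle keeps the last facing.
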(event EventTick
  (params (DeltaSeconds :type Float%20%28single-precision%29))
  (CallFunction|SetMyFlipbook))

(event Input|AxisEvents|InputAxisUpOrDown
  (params (AxisValue :type Float%20%28single-precision%29))
  (Pawn|Input|AddMovementInput "0, 0,1.000000" AxisValue false))

(event Input|AxisEvents|InputAxisRightOrLeft
  (params (AxisValue :type Float%20%28single-precision%29))
  (Pawn|Input|AddMovementInput "1.000000, 0, 0" AxisValue false))

(fn ConstructionScript)

(fn SetMyFlipbook
  (if (or (!= (Input|AxisValues|GetRightOrLeft) 0.0) (!= (Input|AxisValues|GetUpOrDown) 0.0))
    (Variables|Default|SetLastMoveDirection (select (> (Input|AxisValues|GetUpOrDown) 0.0) "NewEnumerator0" (select (< (Input|AxisValues|GetUpOrDown) 0.0) "NewEnumerator1" (select (> (Input|AxisValues|GetRightOrLeft) 0.0) "NewEnumerator3" "NewEnumerator2")))))
  (Sprite|SetFlipbook (Variables|Default|GetSprite) (select (> (Math|Vector|VectorLength (Transformation|GetVelocity)) 0.0) (Utilities|Select :Index (Variables|Default|GetLastMoveDirection) :NewEnumerator0 "/Game/Characters/Crawler/move_up.move_up" :NewEnumerator1 "/Game/Characters/Crawler/move_down.move_down" :NewEnumerator3 "/Game/Characters/Crawler/move_right.move_right" :NewEnumerator2 "/Game/Characters/Crawler/move_left.move_left") (Utilities|Select :Index (Variables|Default|GetLastMoveDirection) :NewEnumerator0 "/Game/Characters/Crawler/idle_up.idle_up" :NewEnumerator1 "/Game/Characters/Crawler/idle_down.idle_down" :NewEnumerator3 "/Game/Characters/Crawler/idle_right.idle_right" :NewEnumerator2 "/Game/Characters/Crawler/idle_left.idle_left"))))